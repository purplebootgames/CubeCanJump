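; Base enemy actor that travels along a straight path and kills the player character on contact.
; On BeginPlay a timeline lerps its location from RealActorSpawner to RealEndPoint, without sweeping.
; When Sphere1 overlaps a BP_GameCharacter, it calls Death on that character and destroys itself.
; The construction script only prints the MyNumber variable.
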(event `self.ReceiveBeginPlay`
  (bind (_direction _alpha) (`Timeline|TN_MoveEnemy`)
    (:`Update`
      (`self.K2_SetActorLocation` (`KismetMathLibrary.VLerp` (`self.K2_GetActorLocation` (`self.RealActorSpawner`)) (`self.K2_GetActorLocation` (`self.RealEndPoint`)) _alpha)))))

(event `self.Sphere1.OnComponentBeginOverlap`
  (params (OverlappedComponent :type "PrimitiveComponent Object Reference") (OtherActor :type "Actor Object Reference") (OtherComp :type "PrimitiveComponent Object Reference") (OtherBodyIndex :type Integer) (bFromSweep :type Boolean) (SweepResult :type "HitResult Structure (by ref)"))
  (bind _asbp_game_character (cast `/Game/Blueprints/BP_GameCharacter` OtherActor))
  (`/Game/Blueprints/BP_GameCharacter.Death` _asbp_game_character)
  (`self.K2_DestroyActor`))

(fn `UserConstructionScript`
  (`KismetSystemLibrary.PrintString` (`KismetStringLibrary.Conv_IntToString` (`self.MyNumber`))))