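; BP_ActorSpawner periodically spawns BP_EnemyBase enemies at its own transform while the player is alive.
; Tick casts the player pawn to BP_GameCharacter and sets the SpawnEnemies flag from its PlayerAlive state.
; A looping timer started on BeginPlay calls SpawnEnemy, which checks that flag and passes EndPoint and ActorSpawner references to each new enemy.
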(event `self.ReceiveTick`
  (params (DeltaSeconds :type "Float (single-precision)"))
  (bind _asbp_game_character (cast `/Game/Blueprints/BP_GameCharacter` (`GameplayStatics.GetPlayerPawn` 0)))
  (if (`/Game/Blueprints/BP_GameCharacter.PlayerAlive` _asbp_game_character)
    (set `self.SpawnEnemies` true)
    (else
      (set `self.SpawnEnemies` false))))

(event `self.ReceiveBeginPlay`
  (`KismetSystemLibrary.K2_SetTimer` null "SpawnEnemy" 2.0 true 1.0))

(fn `SpawnEnemy`
  (if (`self.SpawnEnemies`)
    (`|SpawnActorFromClass` "/Game/Blueprints/BP_EnemyBase.BP_EnemyBase_C" (`self.GetTransform`) "Undefined" "OverrideRootScale" null 0 (`self.EndPoint`) (`self.ActorSpawner`) null)))

(fn `UserConstructionScript`)